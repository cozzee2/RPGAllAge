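; Melee attack component for BP_ThirdPersonCharacter, running a four-step sword and kick montage combo from IA_Attack input.
; AttackIndex picks the next montage, and SwordAttackCombo either continues a buffered attack (SaveAttack) or resets the chain.
; Hits come from a one-shot sphere trace or a timer-looped hand-point sweep with a hit cooldown.
; Both damage "Damageable" actors and play camera shake.
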(event `self.ReceiveBeginPlay`
  (bind _asbp_third_person_character (cast `/Game/ThirdPerson/Blueprints/BP_ThirdPersonCharacter` (`self.GetOwner`)))
  (set `self.CharacterBP` _asbp_third_person_character)
  (set `self.CharacterMesh` (`Character.Mesh` _asbp_third_person_character)))

(event `Attack1`
  ;[0 0 0] 콤보 시스템
  ;;[1 1 1] 공격1
  (`/Engine/EditorBlueprintResources/StandardMacros.DoOnce` false :!label _label
    (:`Completed`
      (`KismetSystemLibrary.Delay` 0.1)
      (`|PlayMontage` (`self.CharacterMesh`) "/Game/Characters/RPG_Character/Animations/SwordAttack/Attack1_Montage.Attack1_Montage"
        (:`then`
          (set `self.AttackIndex` 1)
          (goto _label :!via `Reset`))))))

(event `EnhancedInput|/Game/ThirdPerson/Input/Actions/IA_Attack`
  (params (ActionValue :type Boolean) (ElapsedSeconds :type "Float (double-precision)") (TriggeredSeconds :type "Float (double-precision)") (InputAction :type "InputAction Object Reference" :default "/Game/ThirdPerson/Input/Actions/IA_Attack.IA_Attack"))
  ;[0 0 0] 콤보 시스템
  ;;[1 1 1] 공격클릭함
  (:`Started`
    (if (`self.CanAttack?`)
      (`self.SwardAttack`))))

(event `SwardAttack`
  ;[0 0 0] 콤보 시스템
  ;;[1 1 1] 칼로 공격
  (if (`self.IsAttacking?`)
    (set `self.SaveAttack?` true)
    (else
      (set `self.IsAttacking?` false)
      (switch `int` (`self.AttackIndex`) :!label _label_2
        (:`0`
          (`self.Attack1`))
        (:`1`
          (`self.Attack2`))
        (:`2`
          (`self.Attack3`))
        (:`3`
          (`self.Attack4`))))))

(event `Attack2`
  ;[0 0 0] 콤보 시스템
  ;;[1 1 1] 공격2
  (`/Engine/EditorBlueprintResources/StandardMacros.DoOnce` false :!label _label_3
    (:`Completed`
      (`KismetSystemLibrary.Delay` 0.1)
      (`|PlayMontage` (`self.CharacterMesh`) "/Game/Characters/RPG_Character/Animations/SwordAttack/Attack2_Montage.Attack2_Montage"
        (:`then`
          (set `self.AttackIndex` 2)
          (goto _label_3 :!via `Reset`))))))

(event `SwordAttackCombo`
  ;[0 0 0] 콤보 시스템
  ;;[1 1 1] 콤보계속
  (if (`self.SaveAttack?`)
    (set `self.SaveAttack?` false)
    (goto _label_2)
    (else
      (`self.StopCombo`))))

(event `Attack3`
  ;[0 0 0] 콤보 시스템
  ;;[1 1 1] 공격3
  (`/Engine/EditorBlueprintResources/StandardMacros.DoOnce` false :!label _label_4
    (:`Completed`
      (`KismetSystemLibrary.Delay` 0.1)
      (`|PlayMontage` (`self.CharacterMesh`) "/Game/Characters/RPG_Character/Animations/SwordAttack/Kick_Montage.Kick_Montage"
        (:`then`
          (set `self.AttackIndex` 3)
          (goto _label_4 :!via `Reset`))))))

(event `StopCombo`
  ;[0 0 0] 콤보 시스템
  ;;[1 1 1] 콤보정지함
  (set `self.SaveAttack?` false)
  (set `self.AttackIndex` 0))

(event `Attack4`
  ;[0 0 0] 콤보 시스템
  ;;[1 1 1] 공격4
  (`/Engine/EditorBlueprintResources/StandardMacros.DoOnce` false :!label _label_5
    (:`Completed`
      (`KismetSystemLibrary.Delay` 0.1)
      (`|PlayMontage` (`self.CharacterMesh`) "/Game/Characters/RPG_Character/Animations/SwordAttack/Attack3_Montage.Attack3_Montage"
        (:`then`
          (set `self.AttackIndex` 4)
          (goto _label_5 :!via `Reset`))))))

(event `SphereTrace`
  (bind _returnvalue (`SceneComponent.K2_GetComponentLocation` (`/Game/ThirdPerson/Blueprints/BP_ThirdPersonCharacter.SphereTrace` (`self.CharacterBP`))))
  ;[1 1 1] 스피어트레이스(차기와 뻗기)
  (bind (_outhit _returnvalue_2) (`KismetSystemLibrary.SphereTraceSingle` :`Start` _returnvalue :`End` _returnvalue :`Radius` 25.0 :`TraceChannel` "TraceTypeQuery1" :`DrawDebugType` "ForDuration"))
  (if _returnvalue_2
    (bind (_bblockinghit _binitialoverlap _time _distance _location _impactpoint _normal _impactnormal _physmat _hitactor) (`GameplayStatics.BreakHitResult` _outhit))
    (if (`Actor.ActorHasTag` _hitactor "Damageable")
      (`GameplayStatics.ApplyDamage` _hitactor 10.0)
      (`GameplayStatics.PlayWorldCameraShake` "/Game/Blueprints/BP_HitCameraShake.BP_HitCameraShake_C" _location 0.0 2000.0))))

(event `StartSwordTrace`
  ;[1 1 1] 칼로공격
  (bind _returnvalue (`KismetSystemLibrary.K2_SetTimerDelegate` (delegate `SwordTraceLoop`) 0.001 true))
  (set `self.Sword Trace Loop` _returnvalue))

(event `SwordTraceLoop`
  ;[1 1 1] 칼로공격
  (bind (_outhit _returnvalue) (`KismetSystemLibrary.SphereTraceSingle` :`Start` (`SceneComponent.K2_GetComponentLocation` (`/Game/ThirdPerson/Blueprints/BP_ThirdPersonCharacter.HandPoint_Top` (`self.CharacterBP`))) :`End` (`SceneComponent.K2_GetComponentLocation` (`/Game/ThirdPerson/Blueprints/BP_ThirdPersonCharacter.HandPoint_Bottom` (`self.CharacterBP`))) :`Radius` 12.0 :`TraceChannel` "TraceTypeQuery1" :`DrawDebugType` "ForDuration" :`DrawTime` 0.2))
  (if _returnvalue
    (bind (_bblockinghit _binitialoverlap _time _distance _location _impactpoint _normal _impactnormal _physmat _hitactor) (`GameplayStatics.BreakHitResult` _outhit))
    (if (`Actor.ActorHasTag` _hitactor "Damageable")
      (`/Engine/EditorBlueprintResources/StandardMacros.DoOnce` false :!label _label_6
        (:`Completed`
          (`GameplayStatics.ApplyDamage` _hitactor 10.0)
          (`GameplayStatics.PlayWorldCameraShake` "/Game/Blueprints/BP_HitCameraShake.BP_HitCameraShake_C" _location 0.0 2000.0)
          (`KismetSystemLibrary.Delay` 0.5)
          (goto _label_6 :!via `Reset`))))))

(event `StopSwordTrace`
  ;[1 1 1] 칼로공격
  (`KismetSystemLibrary.K2_ClearAndInvalidateTimerHandle` (`self.Sword Trace Loop`)))