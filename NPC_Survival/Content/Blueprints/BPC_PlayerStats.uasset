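; Player stats component that tracks current and max health and stamina for the third-person character.
; On BeginPlay it caches the owning BP_ThirdPersonCharacter and uses its HUD widget to update the health bar, health text and stamina bar directly after each change.
; Decrease functions return whether the stat is depleted, increases to current values clamp at max, and max values can be raised.
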(event `self.ReceiveBeginPlay`
  (bind _asbp_third_person_character (cast `/Game/ThirdPerson/Blueprints/BP_ThirdPersonCharacter` (`self.GetOwner`)))
  (set `self.PlayerCharacterBP` _asbp_third_person_character))

(fn `DecreaseHealth`
  (params (Damage :type "Float (double-precision)"))
  (returns (`IsPlayerDead?` :type Boolean))
  (bind _hudwidget (`/Game/ThirdPerson/Blueprints/BP_ThirdPersonCharacter.HUDWidget` (`self.PlayerCharacterBP`)))
  (if (not (<= (`self.CurrentHealth`) 0.0))
    (bind _output_get (set `self.CurrentHealth` (- (`self.CurrentHealth`) Damage)))
    (`ProgressBar.SetPercent` (`/Game/UI/WB_HUD.HealthBar` _hudwidget) (/ _output_get (`self.MaxHealth`)))
    (`TextBlock.SetText` (`/Game/UI/WB_HUD.HealthText` _hudwidget) (`KismetTextLibrary.Conv_DoubleToText` (`self.CurrentHealth`) "HalfToEven"))
    (if (<= (`self.CurrentHealth`) 0.0)
      _
      (else
        (return false))))
  (return true))

(fn `DecreaseStamina`
  (params (StaminaDepleted :type "Float (double-precision)"))
  (returns (NotStaminaLeft :type Boolean))
  (if (not (<= (`self.CurrentStamina`) 0.0))
    (set `self.CurrentStamina` (- (`self.CurrentStamina`) StaminaDepleted))
    (`ProgressBar.SetPercent` (`/Game/UI/WB_HUD.StaminaBar` (`/Game/ThirdPerson/Blueprints/BP_ThirdPersonCharacter.HUDWidget` (`self.PlayerCharacterBP`))) (/ (`self.CurrentStamina`) (`self.MaxStamina`)))
    (if (<= (`self.CurrentStamina`) 0.0)
      _
      (else
        (return false))))
  (return true))

(fn `IncreaseHealth`
  (params (AddedHealth :type "Float (double-precision)"))
  (bind _hudwidget (`/Game/ThirdPerson/Blueprints/BP_ThirdPersonCharacter.HUDWidget` (`self.PlayerCharacterBP`)))
  (set `self.CurrentHealth` (+ (`self.CurrentHealth`) AddedHealth))
  (if (> (`self.CurrentHealth`) (`self.MaxHealth`))
    (set `self.CurrentHealth` (`self.MaxHealth`)))
  (`ProgressBar.SetPercent` (`/Game/UI/WB_HUD.HealthBar` _hudwidget) (/ (`self.CurrentHealth`) (`self.MaxHealth`)))
  (`TextBlock.SetText` (`/Game/UI/WB_HUD.HealthText` _hudwidget) (`KismetTextLibrary.Conv_DoubleToText` (`self.CurrentHealth`) "HalfToEven")))

(fn `IncreaseMaxHealth`
  (params (HealthIncremention :type "Float (double-precision)"))
  (bind _hudwidget (`/Game/ThirdPerson/Blueprints/BP_ThirdPersonCharacter.HUDWidget` (`self.PlayerCharacterBP`)))
  (set `self.MaxHealth` (+ (`self.MaxHealth`) HealthIncremention))
  (`ProgressBar.SetPercent` (`/Game/UI/WB_HUD.HealthBar` _hudwidget) (/ (`self.CurrentHealth`) (`self.MaxHealth`)))
  (`TextBlock.SetText` (`/Game/UI/WB_HUD.HealthText` _hudwidget) (`KismetTextLibrary.Conv_DoubleToText` (`self.CurrentHealth`) "HalfToEven")))

(fn `IncreaseMaxStamina`
  (params (AddedStamina :type "Float (double-precision)"))
  (set `self.MaxStamina` (+ (`self.MaxStamina`) AddedStamina))
  (`ProgressBar.SetPercent` (`/Game/UI/WB_HUD.StaminaBar` (`/Game/ThirdPerson/Blueprints/BP_ThirdPersonCharacter.HUDWidget` (`self.PlayerCharacterBP`))) (/ (`self.CurrentStamina`) (`self.MaxStamina`))))

(fn `IncreseStamina`
  (params (AddedStamina :type "Float (double-precision)"))
  (set `self.CurrentStamina` (+ (`self.CurrentStamina`) AddedStamina))
  (if (> (`self.CurrentStamina`) (`self.MaxStamina`))
    (set `self.CurrentStamina` (`self.MaxStamina`)))
  (`ProgressBar.SetPercent` (`/Game/UI/WB_HUD.StaminaBar` (`/Game/ThirdPerson/Blueprints/BP_ThirdPersonCharacter.HUDWidget` (`self.PlayerCharacterBP`))) (/ (`self.CurrentStamina`) (`self.MaxStamina`))))